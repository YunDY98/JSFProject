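; TestAct is a test actor that exercises JSON loading and prints the parsed results on screen at BeginPlay.
; Youtube loads through MyJson, prints its PlayerStruct as pink long-duration text and stores the JsonData.
; My runs a parallel load through MyJson and prints each string derived from CommonStruct.
; BeginPlay then prints every entry returned by ParseJsonSwitching, whose body is outside this graph.
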(event EventBeginPlay
  (CallFunction|Youtube)
  (CallFunction|My)
  (bind _text (Class|MyBlueprintFunctionLibrary|ParseJsonSwitching))
  (for _array_element _text
    (Development|PrintString _array_element)))

(event Collision|EventActorBeginOverlap
  (params (OtherActor :type Actor%20Object%20Reference)))

(event EventTick
  (params (DeltaSeconds :type Float%20%28single-precision%29)))

(fn ConstructionScript)

(fn Youtube
  (bind _myjson (Variables|Default|GetMyJson))
  (Class|MyJsonComponent|FLoadJson _myjson)
  (bind _returnvalue (Class|MyJsonComponent|FPrintFPlayerStruct _myjson (Variables|/Script/MyJson.MyJsonComponent|GetplayerStruct _myjson)))
  (Development|PrintString _returnvalue true true "(R=1.000000,G=0.170517,B=0.926912,A=1.000000)" 22.0)
  (Variables|Default|SetJsonData (Variables|/Script/MyJson.MyJsonComponent|GetJsonData _myjson)))

(fn My
  (bind _myjson (Variables|Default|GetMyJson))
  (Class|MyJsonComponent|MyLoadJson _myjson)
  (bind _returnvalue (Class|MyJsonComponent|MyPrintFPlayerStruct _myjson (Variables|/Script/MyJson.MyJsonComponent|GetCommonStruct _myjson)))
  (for _array_element _returnvalue
    (Development|PrintString _array_element true true "(R=1.000000,G=0.170517,B=0.926912,A=1.000000)" 22.0)))